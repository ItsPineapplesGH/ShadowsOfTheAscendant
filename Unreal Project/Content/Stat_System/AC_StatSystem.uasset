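; Actor component that manages player stats such as health, experience and level in an enum-keyed map.
; Add, Subtract and Set functions write the map, with Add and Subtract triggering checks that clamp Health between zero and MaxHealth.
; Gaining Exp past MaxExp carries over the remainder, raises Level and adds MaxHealth and MaxExp increases from DT_LevelStats, rechecking recursively for multiple level-ups.
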(event Custom|Check%20Min%20Health
  ;[0.15 0.15 0.15 0.5] Check if Player Health Reaches Min or Max Amount
  (if (<= (.Stat%20Value (CallFunction|StatCheck "NewEnumerator5")) 0.0)
    (CallFunction|SetStatValue "NewEnumerator5" 0.0)))

(event Custom|Check%20Max%20Health
  (bind _stat_value (CallFunction|StatCheck "NewEnumerator4"))
  ;[0.15 0.15 0.15 0.5] Check if Player Health Reaches Min or Max Amount
  (if (>= (.Stat%20Value (CallFunction|StatCheck "NewEnumerator5")) _stat_value)
    (CallFunction|SetStatValue "NewEnumerator5" _stat_value)))

(event Custom|Check%20Max%20Xp
  (bind _stat_value (CallFunction|StatCheck "NewEnumerator1"))
  ;[0.15 0.15 0.15 0.5] Check if Player Reaches Max Exp For Gaining A Level
  (if (>= (.Stat%20Value (CallFunction|StatCheck "NewEnumerator2")) _stat_value)
    (CallFunction|SubtractStatValue "NewEnumerator2" _stat_value)
    (CallFunction|AddStatValue "NewEnumerator3" 1.0)
    (bind _returnvalue (Utilities|GetDataTableRow "/Game/Stat_System/DT_LevelStats.DT_LevelStats" (Utilities|String|StringToName (Utilities|String|Append "Level_" (Utilities|String|ToString(Integer) (Class|KismetMathLibrary|ToInt64(Float) (.Stat%20Value (CallFunction|StatCheck "NewEnumerator3")))))))
      (:then
        (CallFunction|AddStatValue "NewEnumerator4" (.MaxHealth (Utilities|Struct|BreakF_StatsList _returnvalue)))
        (CallFunction|AddStatValue "NewEnumerator1" (.MaxExp (Utilities|Struct|BreakF_StatsList _returnvalue)))
        (CallFunction|CheckMaxXp)))))

(fn StatCheck
  (params (Select%20Stat :type Enum_Stats%20Enum :default "NewEnumerator0"))
  (bind _stats (Variables|Default|GetStats))
  (bind (_value _returnvalue) (Utilities|Map|Find _stats Select%20Stat))
  (return _value _returnvalue))

(fn AddStatValue
  (params (Select%20Stat :type Enum_Stats%20Enum :default "NewEnumerator0") (Add%20Value :type Float%20%28double-precision%29))
  (Utilities|Map|Add (Variables|Default|GetStats) Select%20Stat (+ (.Stat%20Value (CallFunction|StatCheck Select%20Stat)) Add%20Value))
  (switch Utilities|FlowControl|Switch|SwitchonEnum_Stats Select%20Stat
    (:NewEnumerator0
      _)
    (:NewEnumerator1
      _)
    (:NewEnumerator2
      (CallFunction|CheckMaxXp))
    (:NewEnumerator3
      _)
    (:NewEnumerator4
      _)
    (:NewEnumerator5
      (CallFunction|CheckMaxHealth)))
  (return (.Stat%20Value (CallFunction|StatCheck Select%20Stat))))

(fn SubtractStatValue
  (params (Select%20Stat :type Enum_Stats%20Enum :default "NewEnumerator0") (Subtracted%20Value :type Float%20%28double-precision%29))
  (Utilities|Map|Add (Variables|Default|GetStats) Select%20Stat (- (.Stat%20Value (CallFunction|StatCheck Select%20Stat)) Subtracted%20Value))
  (switch Utilities|FlowControl|Switch|SwitchonEnum_Stats Select%20Stat
    (:NewEnumerator0
      _)
    (:NewEnumerator1
      _)
    (:NewEnumerator2
      _)
    (:NewEnumerator3
      _)
    (:NewEnumerator4
      _)
    (:NewEnumerator5
      (CallFunction|CheckMinHealth)))
  (return (.Stat%20Value (CallFunction|StatCheck Select%20Stat))))

(fn SetStatValue
  (params (Select%20Stat :type Enum_Stats%20Enum :default "NewEnumerator0") (Set%20Value :type Float%20%28double-precision%29))
  (Utilities|Map|Add (Variables|Default|GetStats) Select%20Stat Set%20Value)
  (switch Utilities|FlowControl|Switch|SwitchonEnum_Stats Select%20Stat
    (:NewEnumerator0
      _)
    (:NewEnumerator1
      _)
    (:NewEnumerator2
      _)
    (:NewEnumerator3
      _)
    (:NewEnumerator4
      _)
    (:NewEnumerator5
      _))
  (return (.Stat%20Value (CallFunction|StatCheck Select%20Stat))))